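; BP_BatteryReceiver is a battery socket that powers a linked actor when a BP_Battery overlaps its collision while empty.
; It destroys that battery and shows its own battery model sliding in, with green frame material and sounds.
; Power on and off events message ActorToWith and toggle filling on an optional LinkedCable.
; The construction script applies the initial HaveBatteryIn state to visuals and sends matching door open or closed messages.
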(event OnComponentBeginOverlap(Battery_Collision)
  (params (OverlappedComponent :type Primitive%20Component%20Object%20Reference) (OtherActor :type Actor%20Object%20Reference) (OtherComp :type Primitive%20Component%20Object%20Reference) (OtherBodyIndex :type Integer) (bFromSweep :type Boolean) (SweepResult :type Hit%20Result%20Structure%20%28by%20ref%29))
  (bind _asbp_battery (Utilities|Casting|CastToBP_Battery OtherActor))
  (if (not (Variables|Main|GetHaveBatteryIn?))
    (CallFunction|TurnPoweron)
    (Physics|SetSimulatePhysics (Variables|/Game/Blueprints/Mechanics/Battery/BP_Battery.BP_Battery_C|GetBatteryMesh _asbp_battery) false)
    (Actor|DestroyActor _asbp_battery)))

(event Custom|SetDoorOpened
  (Class|BPIBatteryEvent|DoorSetDoorOpened(Message) (Variables|Main|GetActorToWith)))

(event Custom|TurnPowerOn
  (bind _returnvalue (Transformation|GetActorLocation))
  (bind _batterymodel (Variables|Default|GetBatteryModel))
  (bind _linkedcable (Variables|Main|GetLinkedCable))
  (Variables|Main|SetHaveBatteryIn? true)
  (Variables|Default|SetPowered true)
  (Rendering|Material|SetMaterial (Variables|Default|GetBatteryReceiverMesh) 0 "/Game/Materials/Kits/Battery/MI_BatteryFrame_Green.MI_BatteryFrame_Green")
  (Rendering|SetVisibility _batterymodel true false)
  (Utilities|FlowControl|Sequence
    (:then_0
      (Components|MoveComponentTo _batterymodel "0.000000,15.428716,42.777065" "0.000000,0.000000,90.000000" false false 0.6 false))
    (:then_1
      (Audio|PlaySoundatLocation "/Game/Sounds/Grabpack/Battery/SW_Battery_PowerOn_01_Cue.SW_Battery_PowerOn_01_Cue" _returnvalue "0, 0, 0" 1.0 1.0 0.0 0 0 0 0)
      (Audio|PlaySoundatLocation "/Game/Sounds/Grabpack/Battery/SW_Battery_LockIn_01_Cue.SW_Battery_LockIn_01_Cue" _returnvalue "0, 0, 0" 1.0 1.0 0.0 0 0 0 0)
      (bind _returnvalue_2 (AddComponent|AddAudioComponent false))
      (bind _output_get (Variables|Default|SetSW_IdleSound _returnvalue_2))
      (Audio|Components|Audio|Play _output_get 0.0))
    (:then_2
      (Class|BPIBatteryEvent|Batteryin(Message) (Variables|Main|GetActorToWith))
      (Utilities|IsValid _linkedcable
        (:Is%20Valid
          (Variables|/Game/Blueprints/BP_Cable/BP_Cable.BP_Cable_C|SetIsFilling? _linkedcable true))))))

(event Custom|TurnPowerOff
  (bind _batterymodel (Variables|Default|GetBatteryModel))
  (bind _linkedcable (Variables|Main|GetLinkedCable))
  (Variables|Main|SetHaveBatteryIn? false)
  (Variables|Default|SetPowered false)
  (Rendering|Material|SetMaterial (Variables|Default|GetBatteryReceiverMesh) 0 "/Game/Materials/Kits/Battery/MI_BatteryFrame.MI_BatteryFrame")
  (Rendering|SetVisibility _batterymodel false false)
  (Utilities|FlowControl|Sequence
    (:then_0
      (Components|MoveComponentTo _batterymodel "0.000000,19.316257,42.777065" "0.000000,0.000000,90.000000" false false 0.6 false))
    (:then_1
      (Audio|PlaySoundatLocation "/Game/Sounds/Grabpack/Battery/SW_Battery_PowerDown_01_Cue.SW_Battery_PowerDown_01_Cue" (Transformation|GetActorLocation) "0, 0, 0" 1.0 1.0 0.0 0 0 0 0)
      (Audio|Components|Audio|Stop (Variables|Default|GetSW_IdleSound)))
    (:then_2
      (Class|BPIBatteryEvent|BatteryOut(Message) (Variables|Main|GetActorToWith))
      (Utilities|IsValid _linkedcable
        (:Is%20Valid
          (Variables|/Game/Blueprints/BP_Cable/BP_Cable.BP_Cable_C|SetIsFilling? _linkedcable false))))))

(event Custom|SetDoorClosed
  (Class|BPIBatteryEvent|DoorSetDoorClosed(Message) (Variables|Main|GetActorToWith)))

(fn ConstructionScript
  (bind _batterymodel (Variables|Default|GetBatteryModel))
  (if (Variables|Main|GetHaveBatteryIn?)
    (Rendering|SetVisibility _batterymodel true false)
    (Variables|Default|SetPowered true)
    (Rendering|Material|SetMaterial (Variables|Default|GetBatteryReceiverMesh) 0 "/Game/Materials/Kits/Battery/MI_BatteryFrame_Green.MI_BatteryFrame_Green")
    (CallFunction|SetDoorOpened)
    (else
      (Rendering|SetVisibility _batterymodel false false)
      (Variables|Default|SetPowered false)
      (Rendering|Material|SetMaterial (Variables|Default|GetBatteryReceiverMesh) 0 "/Game/Materials/Kits/Battery/MI_BatteryFrame.MI_BatteryFrame")
      (CallFunction|SetDoorClosed))))