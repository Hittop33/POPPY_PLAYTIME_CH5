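; A vertically sliding door actor with four mesh variants that opens and closes in response to power, activation and scan events.
; Poweron, PowerOff, ScanningFinished and Activate set IsPowered, then share one toggle that plays a slam sound and moves the door, ignoring requests mid-move.
; IsPowered never gates movement, so even PowerOff flips the door.
; The construction script applies DoorType meshes and positions the door from IsOpened.
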(event EventActivate
  (bind _doortype (Variables|Default|GetDoorType))
  (Variables|Default|SetIsPowered? true)
  (if (not (Variables|Default|GetIsOpeningDoor))
    (Variables|Default|SetIsOpeningDoor true)
    (bind _output_get (Variables|Default|SetIsOpened? (not (Variables|Default|GetIsOpened?))))
    (Audio|PlaySoundatLocation "/Game/Blueprints/Mechanics/Doors/SW_SFX_Graveyard_DoorSlam.SW_SFX_Graveyard_DoorSlam" (Transformation|GetActorLocation) "0, 0, 0" 1.0 1.0 0.0 0 0 0 0)
    (Components|MoveComponentTo (Variables|Default|GetDoor) (Math|Vector|MakeVector (Utilities|Select :Index _doortype :Option%200 -3.0 :Option%201 0.0 :Option%202 -2.0 :Option%203 0.0) 0.0 (select _output_get (Utilities|Select :Index _doortype :Option%200 2.9e+02 :Option%201 2.9e+02 :Option%202 4.9e+02 :Option%203 3e+02) 0.0)) "0, 0, 0" false false 1.5 false)
    (Variables|Default|SetIsOpeningDoor false)))

(event EventPoweron
  (bind _doortype (Variables|Default|GetDoorType))
  (Variables|Default|SetIsPowered? true)
  (if (not (Variables|Default|GetIsOpeningDoor))
    (Variables|Default|SetIsOpeningDoor true)
    (bind _output_get (Variables|Default|SetIsOpened? (not (Variables|Default|GetIsOpened?))))
    (Audio|PlaySoundatLocation "/Game/Blueprints/Mechanics/Doors/SW_SFX_Graveyard_DoorSlam.SW_SFX_Graveyard_DoorSlam" (Transformation|GetActorLocation) "0, 0, 0" 1.0 1.0 0.0 0 0 0 0)
    (Components|MoveComponentTo (Variables|Default|GetDoor) (Math|Vector|MakeVector (Utilities|Select :Index _doortype :Option%200 -3.0 :Option%201 0.0 :Option%202 -2.0 :Option%203 0.0) 0.0 (select _output_get (Utilities|Select :Index _doortype :Option%200 2.9e+02 :Option%201 2.9e+02 :Option%202 4.9e+02 :Option%203 3e+02) 0.0)) "0, 0, 0" false false 1.5 false)
    (Variables|Default|SetIsOpeningDoor false)))

(event EventScanningFinished
  (bind _doortype (Variables|Default|GetDoorType))
  (Variables|Default|SetIsPowered? true)
  (if (not (Variables|Default|GetIsOpeningDoor))
    (Variables|Default|SetIsOpeningDoor true)
    (bind _output_get (Variables|Default|SetIsOpened? (not (Variables|Default|GetIsOpened?))))
    (Audio|PlaySoundatLocation "/Game/Blueprints/Mechanics/Doors/SW_SFX_Graveyard_DoorSlam.SW_SFX_Graveyard_DoorSlam" (Transformation|GetActorLocation) "0, 0, 0" 1.0 1.0 0.0 0 0 0 0)
    (Components|MoveComponentTo (Variables|Default|GetDoor) (Math|Vector|MakeVector (Utilities|Select :Index _doortype :Option%200 -3.0 :Option%201 0.0 :Option%202 -2.0 :Option%203 0.0) 0.0 (select _output_get (Utilities|Select :Index _doortype :Option%200 2.9e+02 :Option%201 2.9e+02 :Option%202 4.9e+02 :Option%203 3e+02) 0.0)) "0, 0, 0" false false 1.5 false)
    (Variables|Default|SetIsOpeningDoor false)))

(event EventPowerOff
  (bind _doortype (Variables|Default|GetDoorType))
  (Variables|Default|SetIsPowered? false)
  (if (not (Variables|Default|GetIsOpeningDoor))
    (Variables|Default|SetIsOpeningDoor true)
    (bind _output_get (Variables|Default|SetIsOpened? (not (Variables|Default|GetIsOpened?))))
    (Audio|PlaySoundatLocation "/Game/Blueprints/Mechanics/Doors/SW_SFX_Graveyard_DoorSlam.SW_SFX_Graveyard_DoorSlam" (Transformation|GetActorLocation) "0, 0, 0" 1.0 1.0 0.0 0 0 0 0)
    (Components|MoveComponentTo (Variables|Default|GetDoor) (Math|Vector|MakeVector (Utilities|Select :Index _doortype :Option%200 -3.0 :Option%201 0.0 :Option%202 -2.0 :Option%203 0.0) 0.0 (select _output_get (Utilities|Select :Index _doortype :Option%200 2.9e+02 :Option%201 2.9e+02 :Option%202 4.9e+02 :Option%203 3e+02) 0.0)) "0, 0, 0" false false 1.5 false)
    (Variables|Default|SetIsOpeningDoor false)))

(fn ConstructionScript
  (bind _door (Variables|Default|GetDoor))
  (bind _doortype (Variables|Default|GetDoorType))
  (bind _doortype_2 (Variables|Default|GetDoorType))
  (Utilities|FlowControl|Sequence
    (:then_0
      (if (Variables|Default|GetIsOpened?)
        (Transformation|SetRelativeLocation _door (Math|Vector|MakeVector (Utilities|Select :Index _doortype_2 :Option%200 -3.0 :Option%201 0.0 :Option%202 -2.0 :Option%203 0.0) 0.0 (Utilities|Select :Index _doortype_2 :Option%200 2.9e+02 :Option%201 2.9e+02 :Option%202 4.9e+02 :Option%203 3e+02)) false false)
        (else
          (Transformation|SetRelativeLocation _door (Math|Vector|MakeVector (Utilities|Select :Index (Variables|Default|GetDoorType) :Option%200 -3.0 :Option%201 0.0 :Option%202 -2.0 :Option%203 0.0) 0.0 0.0) false false))))
    (:then_1
      (Components|StaticMesh|SetStaticMesh _door (Utilities|Select :Index _doortype :Option%200 "/Game/Meshes/ppt5kits/Doors/SlidingDoor/SM_SlidingDoor1PPT4_SM_SlidingDoor_D_mo.SM_SlidingDoor1PPT4_SM_SlidingDoor_D_mo" :Option%201 "/Game/Meshes/ppt5kits/Doors/SlidingDoor1/SM_SlidingDoor2PPT4.SM_SlidingDoor2PPT4" :Option%202 "/Game/Meshes/ppt5kits/Doors/SlidingDoor2/SM_SlidingDoor3PPT4_SM_SlidingDoor_3x5_mo.SM_SlidingDoor3PPT4_SM_SlidingDoor_3x5_mo" :Option%203 "/Game/Meshes/ppt5kits/Doors/SlidingDoor3/SM_SlidingDoor4_SM_SlidingDoor_3x3_A_mo.SM_SlidingDoor4_SM_SlidingDoor_3x3_A_mo")))
    (:then_2
      (Components|StaticMesh|SetStaticMesh (Variables|Default|GetDoorFrame) (Utilities|Select :Index _doortype :Option%200 "/Game/Meshes/ppt5kits/Doors/SlidingDoor/SM_SlidingDoor1PPT4_SM_SlidingDoor_C_Frame_mo.SM_SlidingDoor1PPT4_SM_SlidingDoor_C_Frame_mo" :Option%201 "/Game/Meshes/ppt5kits/Doors/SlidingDoor/SM_SlidingDoor1PPT4_SM_SlidingDoor_C_Frame_mo.SM_SlidingDoor1PPT4_SM_SlidingDoor_C_Frame_mo" :Option%202 "/Game/Meshes/ppt5kits/Doors/SlidingDoor2/SM_SlidingDoor3PPT4_SM_SlidingDoor_3x5_Frame_mo.SM_SlidingDoor3PPT4_SM_SlidingDoor_3x5_Frame_mo" :Option%203 "/Game/Meshes/ppt5kits/Doors/SlidingDoor3/SM_SlidingDoor4_SM_SlidingDoor_3x3_B_mo.SM_SlidingDoor4_SM_SlidingDoor_3x3_B_mo")))))