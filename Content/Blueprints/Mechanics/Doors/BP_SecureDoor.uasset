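; BP_SecureDoor is a rotating metal door that responds to interaction only while powered.
; Power on, scanning finished and activate events set it powered and toggle it, while power off clears power and still toggles it.
; Each toggle plays a sound and tweens the Door component between closed and DoorMaxRotation, ignoring triggers during motion.
; The construction script previews IsOpened using a hardcoded open angle instead of DoorMaxRotation.
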(event EventActivate
  (Variables|Default|SetIsPowered? true)
  (if (not (Variables|Default|GetIsOpeningDoor))
    (Variables|Default|SetIsOpeningDoor true)
    (bind _output_get (Variables|Default|SetIsOpened? (not (Variables|Default|GetIsOpened?))))
    (Audio|PlaySoundatLocation "/Game/Sounds/Doors/Metal/SW_Door_Metal_Rotating_01_Cue.SW_Door_Metal_Rotating_01_Cue" (Transformation|GetActorLocation) "0, 0, 0" 1.0 1.0 0.0 0 0 0 0)
    (Components|MoveComponentTo (Variables|Default|GetDoor) "-80.000000,0.000000,0.000000" (Math|Rotator|MakeRotator 0.0 0.0 (select _output_get (Variables|Default|GetDoorMaxRotation) 0.0)) false false 1.0 true)
    (Variables|Default|SetIsOpeningDoor false)))

(event EventPoweron
  (Variables|Default|SetIsPowered? true)
  (if (not (Variables|Default|GetIsOpeningDoor))
    (Variables|Default|SetIsOpeningDoor true)
    (bind _output_get (Variables|Default|SetIsOpened? (not (Variables|Default|GetIsOpened?))))
    (Audio|PlaySoundatLocation "/Game/Sounds/Doors/Metal/SW_Door_Metal_Rotating_01_Cue.SW_Door_Metal_Rotating_01_Cue" (Transformation|GetActorLocation) "0, 0, 0" 1.0 1.0 0.0 0 0 0 0)
    (Components|MoveComponentTo (Variables|Default|GetDoor) "-80.000000,0.000000,0.000000" (Math|Rotator|MakeRotator 0.0 0.0 (select _output_get (Variables|Default|GetDoorMaxRotation) 0.0)) false false 1.0 true)
    (Variables|Default|SetIsOpeningDoor false)))

(event EventInteraction
  (if (Variables|Default|GetIsPowered?)
    (if (not (Variables|Default|GetIsOpeningDoor))
      (Variables|Default|SetIsOpeningDoor true)
      (bind _output_get (Variables|Default|SetIsOpened? (not (Variables|Default|GetIsOpened?))))
      (Audio|PlaySoundatLocation "/Game/Sounds/Doors/Metal/SW_Door_Metal_Rotating_01_Cue.SW_Door_Metal_Rotating_01_Cue" (Transformation|GetActorLocation) "0, 0, 0" 1.0 1.0 0.0 0 0 0 0)
      (Components|MoveComponentTo (Variables|Default|GetDoor) "-80.000000,0.000000,0.000000" (Math|Rotator|MakeRotator 0.0 0.0 (select _output_get (Variables|Default|GetDoorMaxRotation) 0.0)) false false 1.0 true)
      (Variables|Default|SetIsOpeningDoor false))))

(event EventScanningFinished
  (Variables|Default|SetIsPowered? true)
  (if (not (Variables|Default|GetIsOpeningDoor))
    (Variables|Default|SetIsOpeningDoor true)
    (bind _output_get (Variables|Default|SetIsOpened? (not (Variables|Default|GetIsOpened?))))
    (Audio|PlaySoundatLocation "/Game/Sounds/Doors/Metal/SW_Door_Metal_Rotating_01_Cue.SW_Door_Metal_Rotating_01_Cue" (Transformation|GetActorLocation) "0, 0, 0" 1.0 1.0 0.0 0 0 0 0)
    (Components|MoveComponentTo (Variables|Default|GetDoor) "-80.000000,0.000000,0.000000" (Math|Rotator|MakeRotator 0.0 0.0 (select _output_get (Variables|Default|GetDoorMaxRotation) 0.0)) false false 1.0 true)
    (Variables|Default|SetIsOpeningDoor false)))

(event EventPowerOff
  (Variables|Default|SetIsPowered? false)
  (if (not (Variables|Default|GetIsOpeningDoor))
    (Variables|Default|SetIsOpeningDoor true)
    (bind _output_get (Variables|Default|SetIsOpened? (not (Variables|Default|GetIsOpened?))))
    (Audio|PlaySoundatLocation "/Game/Sounds/Doors/Metal/SW_Door_Metal_Rotating_01_Cue.SW_Door_Metal_Rotating_01_Cue" (Transformation|GetActorLocation) "0, 0, 0" 1.0 1.0 0.0 0 0 0 0)
    (Components|MoveComponentTo (Variables|Default|GetDoor) "-80.000000,0.000000,0.000000" (Math|Rotator|MakeRotator 0.0 0.0 (select _output_get (Variables|Default|GetDoorMaxRotation) 0.0)) false false 1.0 true)
    (Variables|Default|SetIsOpeningDoor false)))

(fn ConstructionScript
  (bind _door (Variables|Default|GetDoor))
  (if (Variables|Default|GetIsOpened?)
    (Transformation|SetRelativeRotation _door "0.000000,-100.000000,0.000000" false false)
    (else
      (Transformation|SetRelativeRotation _door "0, 0, 0" false false))))