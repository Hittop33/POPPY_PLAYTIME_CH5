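; Swinging door with colour variants that toggles open or closed on interaction while powered, or when power, scan and activation events fire.
; ToggleDoor hides prompts, plays a sound and rotates the mesh with MoveComponentTo, using a busy flag against retriggering.
; A sphere overlap highlights the door with an overlay material and shows widgets, including a no-power warning.
; The construction script applies the DoorType material and the initial open or closed rotation.
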(event OnComponentEndOverlap(Sphere)
  (params (OverlappedComponent :type Primitive%20Component%20Object%20Reference) (OtherActor :type Actor%20Object%20Reference) (OtherComp :type Primitive%20Component%20Object%20Reference) (OtherBodyIndex :type Integer))
  (Utilities|Casting|CastToBP_ThirdPersonCharacter OtherActor)
  (Rendering|Material|SetOverlayMaterial (Variables|Components|GetDoorMesh) 0 :!class /Script/Engine.MeshComponent)
  (Rendering|SetVisibility (Variables|Default|GetWidget1) false false)
  (Rendering|SetVisibility (Variables|Default|GetWidget2) false false))

(event OnComponentBeginOverlap(Sphere)
  (params (OverlappedComponent :type Primitive%20Component%20Object%20Reference) (OtherActor :type Actor%20Object%20Reference) (OtherComp :type Primitive%20Component%20Object%20Reference) (OtherBodyIndex :type Integer) (bFromSweep :type Boolean) (SweepResult :type Hit%20Result%20Structure%20%28by%20ref%29))
  (Utilities|Casting|CastToBP_ThirdPersonCharacter OtherActor)
  (Rendering|Material|SetOverlayMaterial (Variables|Components|GetDoorMesh) "/Game/Materials/emmiee_Inst1.emmiee_Inst1" :!class /Script/Engine.MeshComponent)
  (Rendering|SetVisibility (Variables|Default|GetWidget1) true false)
  (if (Variables|Powering|GetNeedPower?)
    (if (not (Variables|Powering|GetIsPowered?))
      (Rendering|SetVisibility (Variables|Default|GetWidget2) true false))))

(event Custom|ToggleDoor
  (if (not (Variables|Default|GetIsOpeningDoor))
    (Rendering|SetVisibility (Variables|Default|GetWidget2) false false)
    (Rendering|SetVisibility (Variables|Default|GetWidget) false false)
    (Variables|Default|SetIsOpeningDoor true)
    (bind _output_get (Variables|Main|SetIsDoorOpened (not (Variables|Main|GetIsDoorOpened))))
    (Audio|PlaySoundatLocation "/Game/Sounds/Doors/Metal/SW_Door_Metal_Rotating_01_Cue.SW_Door_Metal_Rotating_01_Cue" (Transformation|GetActorLocation) "0, 0, 0" 1.0 1.0 0.0 0 0 0 0)
    (Components|MoveComponentTo (Variables|Components|GetDoorMesh) "-56.498962,0.000000,0.000000" (Math|Rotator|MakeRotator 0.0 0.0 (select _output_get (Variables|Default|GetDoorMaxRotation) 0.0)) false false 1.0 true)
    (Variables|Default|SetIsOpeningDoor false)))

(event EventBeginPlay)

(event Collision|EventActorBeginOverlap
  (params (OtherActor :type Actor%20Object%20Reference)))

(event EventTick
  (params (DeltaSeconds :type Float%20%28single-precision%29)))

(event EventActivate
  (Variables|Powering|SetIsPowered? true)
  (if (not (Variables|Default|GetIsOpeningDoor))
    (Rendering|SetVisibility (Variables|Default|GetWidget2) false false)
    (Rendering|SetVisibility (Variables|Default|GetWidget) false false)
    (Variables|Default|SetIsOpeningDoor true)
    (bind _output_get (Variables|Main|SetIsDoorOpened (not (Variables|Main|GetIsDoorOpened))))
    (Audio|PlaySoundatLocation "/Game/Sounds/Doors/Metal/SW_Door_Metal_Rotating_01_Cue.SW_Door_Metal_Rotating_01_Cue" (Transformation|GetActorLocation) "0, 0, 0" 1.0 1.0 0.0 0 0 0 0)
    (Components|MoveComponentTo (Variables|Components|GetDoorMesh) "-56.498962,0.000000,0.000000" (Math|Rotator|MakeRotator 0.0 0.0 (select _output_get (Variables|Default|GetDoorMaxRotation) 0.0)) false false 1.0 true)
    (Variables|Default|SetIsOpeningDoor false)))

(event EventPoweron
  (bind _widget (Variables|Default|GetWidget))
  (Variables|Powering|SetIsPowered? true)
  (Utilities|FlowControl|Sequence
    (:then_0
      (if (not (Variables|Default|GetIsOpeningDoor))
        (Rendering|SetVisibility (Variables|Default|GetWidget2) false false :!label _label)
        (Rendering|SetVisibility _widget false false)
        (Variables|Default|SetIsOpeningDoor true)
        (bind _output_get (Variables|Main|SetIsDoorOpened (not (Variables|Main|GetIsDoorOpened))))
        (Audio|PlaySoundatLocation "/Game/Sounds/Doors/Metal/SW_Door_Metal_Rotating_01_Cue.SW_Door_Metal_Rotating_01_Cue" (Transformation|GetActorLocation) "0, 0, 0" 1.0 1.0 0.0 0 0 0 0)
        (Components|MoveComponentTo (Variables|Components|GetDoorMesh) "-56.498962,0.000000,0.000000" (Math|Rotator|MakeRotator 0.0 0.0 (select _output_get (Variables|Default|GetDoorMaxRotation) 0.0)) false false 1.0 true)
        (Variables|Default|SetIsOpeningDoor false)))
    (:then_1
      (if (Class|PrimitiveComponent|IsOverlappingComponent (Variables|/Script/Engine.Character|GetCapsuleComponent (Game|GetPlayerCharacter 1)) (Variables|Default|GetSphere))
        (Rendering|SetVisibility _widget true false)))
    (:then_2
      (goto _label))))

(event EventInteraction
  (if (Variables|Powering|GetIsPowered?)
    (if (not (Variables|Default|GetIsOpeningDoor))
      (Rendering|SetVisibility (Variables|Default|GetWidget2) false false)
      (Rendering|SetVisibility (Variables|Default|GetWidget) false false)
      (Variables|Default|SetIsOpeningDoor true)
      (bind _output_get (Variables|Main|SetIsDoorOpened (not (Variables|Main|GetIsDoorOpened))))
      (Audio|PlaySoundatLocation "/Game/Sounds/Doors/Metal/SW_Door_Metal_Rotating_01_Cue.SW_Door_Metal_Rotating_01_Cue" (Transformation|GetActorLocation) "0, 0, 0" 1.0 1.0 0.0 0 0 0 0)
      (Components|MoveComponentTo (Variables|Components|GetDoorMesh) "-56.498962,0.000000,0.000000" (Math|Rotator|MakeRotator 0.0 0.0 (select _output_get (Variables|Default|GetDoorMaxRotation) 0.0)) false false 1.0 true)
      (Variables|Default|SetIsOpeningDoor false))))

(event EventScanningFinished
  (Variables|Powering|SetIsPowered? true)
  (if (not (Variables|Default|GetIsOpeningDoor))
    (Rendering|SetVisibility (Variables|Default|GetWidget2) false false)
    (Rendering|SetVisibility (Variables|Default|GetWidget) false false)
    (Variables|Default|SetIsOpeningDoor true)
    (bind _output_get (Variables|Main|SetIsDoorOpened (not (Variables|Main|GetIsDoorOpened))))
    (Audio|PlaySoundatLocation "/Game/Sounds/Doors/Metal/SW_Door_Metal_Rotating_01_Cue.SW_Door_Metal_Rotating_01_Cue" (Transformation|GetActorLocation) "0, 0, 0" 1.0 1.0 0.0 0 0 0 0)
    (Components|MoveComponentTo (Variables|Components|GetDoorMesh) "-56.498962,0.000000,0.000000" (Math|Rotator|MakeRotator 0.0 0.0 (select _output_get (Variables|Default|GetDoorMaxRotation) 0.0)) false false 1.0 true)
    (Variables|Default|SetIsOpeningDoor false)))

(event EventPowerOff
  (Variables|Powering|SetIsPowered? false)
  (if (not (Variables|Default|GetIsOpeningDoor))
    (Rendering|SetVisibility (Variables|Default|GetWidget2) false false)
    (Rendering|SetVisibility (Variables|Default|GetWidget) false false)
    (Variables|Default|SetIsOpeningDoor true)
    (bind _output_get (Variables|Main|SetIsDoorOpened (not (Variables|Main|GetIsDoorOpened))))
    (Audio|PlaySoundatLocation "/Game/Sounds/Doors/Metal/SW_Door_Metal_Rotating_01_Cue.SW_Door_Metal_Rotating_01_Cue" (Transformation|GetActorLocation) "0, 0, 0" 1.0 1.0 0.0 0 0 0 0)
    (Components|MoveComponentTo (Variables|Components|GetDoorMesh) "-56.498962,0.000000,0.000000" (Math|Rotator|MakeRotator 0.0 0.0 (select _output_get (Variables|Default|GetDoorMaxRotation) 0.0)) false false 1.0 true)
    (Variables|Default|SetIsOpeningDoor false)))

(fn ConstructionScript
  (bind _doormesh (Variables|Components|GetDoorMesh))
  (Utilities|FlowControl|Sequence
    (:then_0
      (for _array_element (Utilities|Array|MakeArray (Variables|Components|GetFrameMesh) (Variables|Components|GetDoorMesh))
        (Rendering|Material|SetMaterial _array_element 0 (Utilities|Select :Index (Variables|Main|GetDoorType) :Option%200 "/Game/Textures/Kits/Doors/T_Door_A_Blue_DIF_Mat.T_Door_A_Blue_DIF_Mat" :Option%201 "/Game/Textures/Kits/Doors/T_Door_A_Grey_DIF_Mat.T_Door_A_Grey_DIF_Mat" :Option%202 "/Game/Textures/Kits/Doors/T_Door_A_Red_DIF_Mat.T_Door_A_Red_DIF_Mat" :Option%203 "/Game/Textures/Kits/Doors/T_Door_A_Yellow_DIF_Mat.T_Door_A_Yellow_DIF_Mat"))))
    (:then_1
      (if (Variables|Main|GetIsDoorOpened)
        (Transformation|SetRelativeRotation _doormesh "0.000000,-100.000000,0.000000" false false)
        (else
          (Transformation|SetRelativeRotation _doormesh "0, 0, 0" false false))))))