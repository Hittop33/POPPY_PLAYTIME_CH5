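; Keycard console that activates a linked actor when the player interacts while holding the keycard matching its KeyCardValue.
; The Construction Script picks console material and card mesh from that value.
; An overlap sphere toggles the prompt widget, and Interaction checks the character's KeyCards array by index.
; A one-time insertion animates the card with a timeline and sounds, then sends ActivateMessage to ActorToActivate after delays.
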(event OnComponentBeginOverlap(Sphere)
  (params (OverlappedComponent :type Primitive%20Component%20Object%20Reference) (OtherActor :type Actor%20Object%20Reference) (OtherComp :type Primitive%20Component%20Object%20Reference) (OtherBodyIndex :type Integer) (bFromSweep :type Boolean) (SweepResult :type Hit%20Result%20Structure%20%28by%20ref%29))
  (Utilities|Casting|CastToBP_ThirdPersonCharacter OtherActor)
  (Rendering|SetVisibility (Variables|Default|GetWidget) true false))

(event OnComponentEndOverlap(Sphere)
  (params (OverlappedComponent :type Primitive%20Component%20Object%20Reference) (OtherActor :type Actor%20Object%20Reference) (OtherComp :type Primitive%20Component%20Object%20Reference) (OtherBodyIndex :type Integer))
  (Utilities|Casting|CastToBP_ThirdPersonCharacter OtherActor)
  (Rendering|SetVisibility (Variables|Default|GetWidget) false false))

(event Custom|KeyCardIsInserted
  (bind _key_card (Variables|Default|GetKey%20Card))
  (if (not (Variables|Default|GetKeyCardIsInserted?))
    (Variables|Default|SetKeyCardIsInserted? true)
    (Rendering|SetVisibility _key_card true false)
    (Development|PrintString "")
    (Audio|PlaySound2D "/Game/Blueprints/Mechanics/KeyCards/SW_SFX_Keycard_Insert.SW_SFX_Keycard_Insert" 1.0 1.0 0.0 0 0)
    (bind _value (Timeline|KeyCardAnimation Play)
      (:Update
        (Transformation|SetRelativeLocation (Variables|Default|GetKey%20Card) (Math|Vector|Lerp(Vector) (Variables|Default|Get1) (Variables|Default|Get2) _value) false false)
        (Utilities|FlowControl|Delay 0.5)
        (Rendering|SetVisibility _key_card false false)
        (Audio|PlaySound2D "/Game/Blueprints/Mechanics/KeyCards/SW_SFX_Keycard_Beep.SW_SFX_Keycard_Beep" 1.0 1.0 0.0 0 0)
        (Utilities|FlowControl|Delay 1.0)
        (Class|BPIKeyCardsDoors|Activate(Message) (Variables|Default|GetActor%20To%20Activate))))))

(event EventInteraction
  (bind _asbp_third_person_character (Utilities|Casting|CastToBP_ThirdPersonCharacter (Game|GetPlayerCharacter 0)))
  (bind (_array_element _array_index) (Utilities|Array|ForEachLoopwithBreak (Variables|/Game/ThirdPerson/Blueprints/BP_ThirdPersonCharacter.BP_ThirdPersonCharacter_C|GetKey%20Cards _asbp_third_person_character) :!label _label)
    (:LoopBody
      (if (and _array_element (== _array_index (Variables|Default|GetKeyCard%20Value)))
        (CallFunction|KeyCardIsInserted)
        (goto _label Break)
        (else
          (Development|PrintString ""))))))

(fn ConstructionScript
  (bind _keycard_value (Variables|Default|GetKeyCard%20Value))
  (Utilities|FlowControl|Sequence
    (:then_0
      (Rendering|Material|SetMaterial (Variables|Default|GetConsolesKC) 0 (Utilities|Select :Index _keycard_value :Option%200 "/Game/Blueprints/Mechanics/KeyCards/SM/ConsolsKC/MI_ConsolR.MI_ConsolR" :Option%201 "/Game/Blueprints/Mechanics/KeyCards/SM/ConsolsKC/MI_ConsolB.MI_ConsolB" :Option%202 "/Game/Blueprints/Mechanics/KeyCards/SM/ConsolsKC/MI_ConsolY.MI_ConsolY" :Option%203 "/Game/Blueprints/Mechanics/KeyCards/SM/ConsolsKC/MI_ConsolG.MI_ConsolG" :Option%204 "/Game/Blueprints/Mechanics/KeyCards/SM/ConsolsKC/MI_ConsolP.MI_ConsolP" :Option%205 "/Game/Blueprints/Mechanics/KeyCards/SM/ConsolsKC/MI_ConsolB.MI_ConsolB")))
    (:then_1
      (Components|StaticMesh|SetStaticMesh (Variables|Default|GetKey%20Card) (Utilities|Select :Index _keycard_value :Option%200 "/Game/Blueprints/Mechanics/KeyCards/SM/RedKeyCard.RedKeyCard" :Option%201 "/Game/Blueprints/Mechanics/KeyCards/SM/BlueKeyCard.BlueKeyCard" :Option%202 "/Game/Blueprints/Mechanics/KeyCards/SM/YellowKeyCard.YellowKeyCard" :Option%203 "/Game/Blueprints/Mechanics/KeyCards/SM/GreenKeyCard.GreenKeyCard" :Option%204 "/Game/Blueprints/Mechanics/KeyCards/SM/PurpleKeyCard.PurpleKeyCard" :Option%205 "/Game/Blueprints/Mechanics/KeyCards/SM/OrangeKeyCard.OrangeKeyCard")))))