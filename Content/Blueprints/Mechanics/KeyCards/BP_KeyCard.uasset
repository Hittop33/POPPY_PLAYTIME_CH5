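; Key card pickup in six colours, with the construction script choosing the static mesh from KeyCardType.
; The player entering its sphere turns on an overlay material highlight and a widget; leaving clears both.
; Interaction runs PickUp, which inserts true into the character's KeyCards at the card type's index (an Insert, not a Set).
; After a short delay it plays a 2D sound and destroys itself.
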(event OnComponentBeginOverlap(Sphere)
  (params (OverlappedComponent :type Primitive%20Component%20Object%20Reference) (OtherActor :type Actor%20Object%20Reference) (OtherComp :type Primitive%20Component%20Object%20Reference) (OtherBodyIndex :type Integer) (bFromSweep :type Boolean) (SweepResult :type Hit%20Result%20Structure%20%28by%20ref%29))
  (Utilities|Casting|CastToBP_ThirdPersonCharacter OtherActor)
  (Rendering|Material|SetOverlayMaterial (Variables|Default|GetKeyCard) "/Game/Materials/emmiee_Inst1.emmiee_Inst1" :!class /Script/Engine.MeshComponent)
  (Rendering|SetVisibility (Variables|Default|GetWidget) true false))

(event OnComponentEndOverlap(Sphere)
  (params (OverlappedComponent :type Primitive%20Component%20Object%20Reference) (OtherActor :type Actor%20Object%20Reference) (OtherComp :type Primitive%20Component%20Object%20Reference) (OtherBodyIndex :type Integer))
  (Utilities|Casting|CastToBP_ThirdPersonCharacter OtherActor)
  (Rendering|Material|SetOverlayMaterial (Variables|Default|GetKeyCard) 0 :!class /Script/Engine.MeshComponent)
  (Rendering|SetVisibility (Variables|Default|GetWidget) false false))

(event Custom|Pick%20Up
  (bind _asbp_third_person_character (Utilities|Casting|CastToBP_ThirdPersonCharacter (Game|GetPlayerCharacter 0)))
  (Utilities|Array|Insert (Variables|/Game/ThirdPerson/Blueprints/BP_ThirdPersonCharacter.BP_ThirdPersonCharacter_C|GetKey%20Cards _asbp_third_person_character) true (Variables|Default|GetKeyCardType))
  (Development|PrintString "")
  (Utilities|FlowControl|Delay 0.2)
  (Audio|PlaySound2D "/Game/Blueprints/Mechanics/KeyCards/0221__1_.0221__1_" 1.0 1.0 0.0 0 0)
  (Actor|DestroyActor))

(event EventInteraction
  (CallFunction|PickUp))

(fn ConstructionScript
  (Components|StaticMesh|SetStaticMesh (Variables|Default|GetKeyCard) (Utilities|Select :Index (Variables|Default|GetKeyCardType) :Option%200 "/Game/Blueprints/Mechanics/KeyCards/SM/RedKeyCard.RedKeyCard" :Option%201 "/Game/Blueprints/Mechanics/KeyCards/SM/BlueKeyCard.BlueKeyCard" :Option%202 "/Game/Blueprints/Mechanics/KeyCards/SM/YellowKeyCard.YellowKeyCard" :Option%203 "/Game/Blueprints/Mechanics/KeyCards/SM/GreenKeyCard.GreenKeyCard" :Option%204 "/Game/Blueprints/Mechanics/KeyCards/SM/PurpleKeyCard.PurpleKeyCard" :Option%205 "/Game/Blueprints/Mechanics/KeyCards/SM/OrangeKeyCard.OrangeKeyCard")))