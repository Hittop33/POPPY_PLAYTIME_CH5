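; Lever actor that the player throws with a hand to trigger a linked actor.
; A timeline rolls the switch, reversing on cancel; on finish, if the player's opening flag is still set, it marks itself opened and messages the linked actor after a delay.
; Events toggle the blue and rocket hand meshes, with the blue one also anchoring the player's left-hand cable.
; The construction script poses the switch from the opened state.
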(event Custom|Opening
  (bind _playerref (Variables|Default|GetPlayerRef))
  (bind _alpha (Timeline|TL_OpenLever PlayFromStart)
    (:Update
      (Transformation|SetRelativeRotation (Variables|Default|GetSwitchModel) (Math|Rotator|MakeRotator (Math|Float|Lerp -4e+01 4e+01 _alpha) 0.0 0.0) false false))
    (:Finished
      (if (Variables|/Game/ThirdPerson/Blueprints/BP_ThirdPersonCharacter.BP_ThirdPersonCharacter_C|GetIsLeverOpeningInProcess? _playerref)
        (Variables|Default|SetIsOpened? true)
        (Utilities|FlowControl|Delay (Variables|Default|GetDelayToOpenTheActor))
        (Class|BPILeverEvents|LeverOpen(Message) (Variables|Default|GetActorToWith))
        (Variables|/Game/ThirdPerson/Blueprints/BP_ThirdPersonCharacter.BP_ThirdPersonCharacter_C|SetIsLeverOpeningInProcess? _playerref false)
        (else
          (Development|PrintString "LeverOpeningNOTinProcess" true true "(R=1.000000,G=0.000000,B=0.413570,A=1.000000)"))))))

(event Custom|CancelledOpening
  (bind _playerref (Variables|Default|GetPlayerRef))
  (bind _alpha (Timeline|TL_OpenLever Reverse)
    (:Update
      (Transformation|SetRelativeRotation (Variables|Default|GetSwitchModel) (Math|Rotator|MakeRotator (Math|Float|Lerp -4e+01 4e+01 _alpha) 0.0 0.0) false false))
    (:Finished
      (if (Variables|/Game/ThirdPerson/Blueprints/BP_ThirdPersonCharacter.BP_ThirdPersonCharacter_C|GetIsLeverOpeningInProcess? _playerref)
        (Variables|Default|SetIsOpened? true)
        (Utilities|FlowControl|Delay (Variables|Default|GetDelayToOpenTheActor))
        (Class|BPILeverEvents|LeverOpen(Message) (Variables|Default|GetActorToWith))
        (Variables|/Game/ThirdPerson/Blueprints/BP_ThirdPersonCharacter.BP_ThirdPersonCharacter_C|SetIsLeverOpeningInProcess? _playerref false)
        (else
          (Development|PrintString "LeverOpeningNOTinProcess" true true "(R=1.000000,G=0.000000,B=0.413570,A=1.000000)"))))))

(event Custom|SetVisibility_AllHandsOFF
  (Rendering|SetVisibility (Variables|Default|GetHand) false false))

(event Custom|SetVisibility_BlueOFF
  (Rendering|SetVisibility (Variables|Default|GetHand) false false))

(event Custom|SetVisibility_RocketOFF
  (Rendering|SetVisibility (Variables|Default|GetHandRocket) false false))

(event Custom|SetVisibility_BlueON
  (bind _hand (Variables|Default|GetHand))
  (Rendering|SetVisibility _hand true false)
  (bind _asbp_third_person_character (Utilities|Casting|CastToBP_ThirdPersonCharacter (Game|GetPlayerCharacter 0)))
  (Class|CableComponent|SetAttachEndtoComponent (Variables|/Game/ThirdPerson/Blueprints/BP_ThirdPersonCharacter.BP_ThirdPersonCharacter_C|GetCableLeftHand _asbp_third_person_character) _hand "None"))

(event Custom|SetVisibility_RocketON
  (Rendering|SetVisibility (Variables|Default|GetHandRocket) true false))

(event EventBeginPlay
  (bind _asbp_third_person_character (Utilities|Casting|CastToBP_ThirdPersonCharacter (Game|GetPlayerCharacter 0)))
  (Variables|Default|SetPlayerRef _asbp_third_person_character))

(fn ConstructionScript
  (bind _switchmodel (Variables|Default|GetSwitchModel))
  (Utilities|FlowControl|Sequence
    (:then_0
      (if (Variables|Default|GetIsOpened?)
        (Transformation|SetRelativeLocationAndRotation _switchmodel "0.000000,5.567757,13.965023" "0.000000,0.000000,40.000000" false false)
        (else
          (Transformation|SetRelativeLocationAndRotation _switchmodel "0.000000,5.567757,13.965023" "0.000000,0.000000,-40.000000" false false))))))