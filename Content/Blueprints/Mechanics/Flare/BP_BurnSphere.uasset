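; BP_BurnSphere is a flare projectile that flies to where the player camera is aimed and burns there briefly.
; On BeginPlay it line-traces along the camera's forward vector, then moves its Collision component to the hit over a distance-scaled time.
; It then plays impact and burning sounds, spawns fire at the hit and smoke without a set location, and disables physics.
; After a delay it destroys both emitters and itself.
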(event EventBeginPlay
  (bind _returnvalue (Game|GetPlayerCameraManager 0))
  (bind _returnvalue_2 (Transformation|GetActorLocation _returnvalue))
  (bind (_outhit _returnvalue_3) (Collision|LineTraceByChannel _returnvalue_2 (+ _returnvalue_2 (* (Transformation|GetActorForwardVector _returnvalue) 100000)) "TraceTypeQuery1" false 0 "None"))
  (if _returnvalue_3
    (Utilities|FlowControl|Delay 0.005)
    (Components|MoveComponentTo (Variables|Default|GetCollision) (.Location (Collision|BreakHitResult _outhit)) (Transformation|GetWorldRotation (Variables|Default|GetCollision)) false false (/ (.Distance (Collision|BreakHitResult _outhit)) 8e+03) false)
    (Audio|PlaySoundatLocation "/Game/Sounds/Grabpack/Flare/SW_Flare_Impact_01_Cue.SW_Flare_Impact_01_Cue" (.Location (Collision|BreakHitResult _outhit)) "0, 0, 0" 1.0 1.0 0.0 0 0 0 0)
    (Audio|PlaySoundatLocation "/Game/Sounds/Grabpack/Flare/SW_Flare_Burning_LOOP_01_Cue.SW_Flare_Burning_LOOP_01_Cue" (.Location (Collision|BreakHitResult _outhit)) "0, 0, 0" 1.0 1.0 0.0 0 0 0 0)
    (bind _returnvalue_4 (Effects|SpawnEmitteratLocation "/Game/StarterContent/Particles/P_Fire.P_Fire" (.Location (Collision|BreakHitResult _outhit)) "0, 0, 0" "0.300000,0.300000,0.300000"))
    (bind _returnvalue_5 (Effects|SpawnEmitteratLocation "/Game/StarterContent/Particles/P_Smoke.P_Smoke" "0, 0, 0" "0, 0, 0" "0.700000,0.700000,0.700000"))
    (Physics|SetSimulatePhysics (Variables|Default|GetCollision) false)
    (Utilities|FlowControl|Delay 8.0)
    (Components|DestroyComponent _returnvalue_4)
    (Components|DestroyComponent _returnvalue_5)
    (Actor|DestroyActor)))

(fn ConstructionScript)