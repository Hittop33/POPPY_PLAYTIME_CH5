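; BP_PuzzlePole is an electric puzzle pole that the third-person character charges by touching it with a hand attached to a power receiver.
; Entering CollisionPlayer sets IsPowered and leaving clears it, each with a 2D charge or discharge sound.
; Both changes require the character's referenced power source to be unpowered and either hand attached.
; The end-overlap power check reads the character cast from the begin-overlap event.
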(event OnComponentBeginOverlap(CollisionPlayer)
  (params (OverlappedComponent :type Primitive%20Component%20Object%20Reference) (OtherActor :type Actor%20Object%20Reference) (OtherComp :type Primitive%20Component%20Object%20Reference) (OtherBodyIndex :type Integer) (bFromSweep :type Boolean) (SweepResult :type Hit%20Result%20Structure%20%28by%20ref%29))
  (bind _asbp_third_person_character (Utilities|Casting|CastToBP_ThirdPersonCharacter OtherActor))
  (if (not (Variables|/Game/Blueprints/Mechanics/Poles/BP_PowerSource.BP_PowerSource_C|GetIsPowered (Variables|/Game/ThirdPerson/Blueprints/BP_ThirdPersonCharacter.BP_ThirdPersonCharacter_C|GetBP_PowerSourceRef _asbp_third_person_character)))
    (if (Variables|/Game/ThirdPerson/Blueprints/BP_ThirdPersonCharacter.BP_ThirdPersonCharacter_C|GetIsLeftHandAttachedToPowerReceiver? _asbp_third_person_character)
      (Development|PrintString "" :!label _label)
      (Variables|Main|SetIsPowered? true)
      (Audio|PlaySound2D "/Game/Sounds/PowerPoles/SW_Conduit_ElectricPole_Charged_Cue.SW_Conduit_ElectricPole_Charged_Cue" 1.0 1.0 0.0 0 0)
      (elif (Variables|/Game/ThirdPerson/Blueprints/BP_ThirdPersonCharacter.BP_ThirdPersonCharacter_C|GetIsRightHandAttachedToPowerReceiver? _asbp_third_person_character)
        (goto _label)
        (else
          (Development|PrintString ""))))))

(event OnComponentEndOverlap(CollisionPlayer)
  (params (OverlappedComponent :type Primitive%20Component%20Object%20Reference) (OtherActor :type Actor%20Object%20Reference) (OtherComp :type Primitive%20Component%20Object%20Reference) (OtherBodyIndex :type Integer))
  (bind _asbp_third_person_character (Utilities|Casting|CastToBP_ThirdPersonCharacter OtherActor))
  (if (not (Variables|/Game/Blueprints/Mechanics/Poles/BP_PowerSource.BP_PowerSource_C|GetIsPowered (Variables|/Game/ThirdPerson/Blueprints/BP_ThirdPersonCharacter.BP_ThirdPersonCharacter_C|GetBP_PowerSourceRef (stale OnComponentBeginOverlap(CollisionPlayer) _asbp_third_person_character))))
    (if (Variables|/Game/ThirdPerson/Blueprints/BP_ThirdPersonCharacter.BP_ThirdPersonCharacter_C|GetIsLeftHandAttachedToPowerReceiver? _asbp_third_person_character)
      (Variables|Main|SetIsPowered? false :!label _label)
      (Audio|PlaySound2D "/Game/Sounds/PowerPoles/SW_Conduit_ElectricPole_Discharged_Cue.SW_Conduit_ElectricPole_Discharged_Cue" 1.0 1.0 0.0 0 0)
      (elif (Variables|/Game/ThirdPerson/Blueprints/BP_ThirdPersonCharacter.BP_ThirdPersonCharacter_C|GetIsRightHandAttachedToPowerReceiver? _asbp_third_person_character)
        (goto _label)
        (else
          (Development|PrintString ""))))))

(event EventBeginPlay)

(event Collision|EventActorBeginOverlap
  (params (OtherActor :type Actor%20Object%20Reference)))

(event EventTick
  (params (DeltaSeconds :type Float%20%28single-precision%29)))

(fn ConstructionScript)