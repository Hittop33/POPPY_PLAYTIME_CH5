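; Power source actor in a pole-and-cable puzzle that passes power from its linked pole into its linked cable.
; FillCable checks whether the linked pole is powered, then marks itself powered and, if the cable is valid, starts it filling.
; That success also plays the puzzle-complete sound and stops the player character's electric sound.
; It has no active Tick or overlap logic; FillCable is its only working event.
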(event Custom|FillCable
  (bind _linked_cable (Variables|Main|GetLinked%20Cable))
  (bind _asbp_third_person_character (Utilities|Casting|CastToBP_ThirdPersonCharacter (Game|GetPlayerCharacter 0)))
  (if (Variables|/Game/Blueprints/Mechanics/Poles/BP_PuzzlePole.BP_PuzzlePole_C|GetIsPowered? (Variables|Default|GetLinked%20Pole))
    (Variables|Main|SetIsPowered true)
    (Utilities|IsValid _linked_cable
      (:Is%20Valid
        (Variables|/Game/Blueprints/BP_Cable/BP_Cable.BP_Cable_C|SetIsFilling? _linked_cable true)
        (Development|PrintString "Flling Cable. Puzzle is Completed")
        (Audio|PlaySound2D "/Game/Sounds/Grabpack/PowerPoles/SW_PuzzleComplete_STEREO_Cue1.SW_PuzzleComplete_STEREO_Cue1" 1.0 1.0 0.0 0 0)
        (Audio|Components|Audio|Stop (Variables|/Game/ThirdPerson/Blueprints/BP_ThirdPersonCharacter.BP_ThirdPersonCharacter_C|GetSW_ElectricSound _asbp_third_person_character))))
    (else
      (Development|PrintString "NOT Powered"))))

(event EventBeginPlay)

(event Collision|EventActorBeginOverlap
  (params (OtherActor :type Actor%20Object%20Reference)))

(event EventTick
  (params (DeltaSeconds :type Float%20%28single-precision%29)))

(fn ConstructionScript)