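; Blue left GrabPack hand actor that snaps onto the interactable the player grabs and can show a held battery.
; Per-target events offset the hand mesh, attach it to the scanner, grab hook, battery receiver, lever, door or power receiver/source, and re-end the left cable on it.
; Most targets come from player character references, and most set a looping grip animation.
; A reversible timeline nudges the hand for lever pulls.
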(event Custom|VisibilityHandMeshBatteryON
  ;[0 1 0.1715] Battery
  (Components|Animation|PlayAnimation (Variables|Default|GetSK_GrabpackHand_DefaultOriginalScrewed_Blue) "/Game/Hand/SK_Hand_Grab_GrabHook_Montage.SK_Hand_Grab_GrabHook_Montage" true)
  (Rendering|SetVisibility (Variables|Default|GetBatteryMesh) true false)
  (Variables|Default|SetHaveBattery? true))

(event Custom|VisibilityHandMeshBatteryOFF
  ;[0 1 0.1715] Battery
  (Rendering|SetVisibility (Variables|Default|GetBatteryMesh) false false)
  (Variables|Default|SetHaveBattery? false))

(event Custom|Hand_SetOFF
  ;[1 0.03075 0.06059] AttachHandToLever
  (Rendering|SetVisibility (Variables|Default|GetSK_GrabpackHand_DefaultOriginalScrewed_Blue) false false))

(event Custom|Hand_SetON
  ;[1 0.03075 0.06059] AttachHandToLever
  (Rendering|SetVisibility (Variables|Default|GetSK_GrabpackHand_DefaultOriginalScrewed_Blue) true false))

(event Custom|AttachHandToDoor
  (bind _sk_grabpackhand_defaultoriginalscrewed_blue (Variables|Default|GetSK_GrabpackHand_DefaultOriginalScrewed_Blue))
  (bind _sk_grabpackhand_defaultoriginalscrewed_blue_2 (Variables|Default|GetSK_GrabpackHand_DefaultOriginalScrewed_Blue))
  (bind _relativerotation (Variables|/Script/Engine.SceneComponent|GetRelativeRotation _sk_grabpackhand_defaultoriginalscrewed_blue))
  (bind _relativelocation (Variables|/Script/Engine.SceneComponent|GetRelativeLocation _sk_grabpackhand_defaultoriginalscrewed_blue))
  ;[1 0.991 0] AttachHandToDoor
  (Transformation|AddRelativeRotation _sk_grabpackhand_defaultoriginalscrewed_blue_2 (Math|Rotator|MakeRotator (.roll _relativerotation) (.pitch _relativerotation) (.yaw _relativerotation)) false false)
  (Transformation|AddRelativeLocation _sk_grabpackhand_defaultoriginalscrewed_blue_2 (Math|Vector|MakeVector (+ (.x _relativelocation) 95.0) (+ (.y _relativelocation) 17.0) (+ (.z _relativelocation) 105.0)) false false)
  (Components|Animation|PlayAnimation (Variables|Default|GetSK_GrabpackHand_DefaultOriginalScrewed_Blue) "/Game/Hand/SK_GrabpackHand_DefaultOriginalScrewed_Blue_Anim_Armature_handL_grab_smallstraightedge_Anim.SK_GrabpackHand_DefaultOriginalScrewed_Blue_Anim_Armature_handL_grab_smallstraightedge_Anim" true)
  (Transformation|AttachComponentToComponent (Variables|Default|GetSK_GrabpackHand_DefaultOriginalScrewed_Blue) (Variables|/Game/Blueprints/Mechanics/Doors/BP_Door.BP_Door_C|GetDoorMesh (Variables|/Game/ThirdPerson/Blueprints/BP_ThirdPersonCharacter.BP_ThirdPersonCharacter_C|GetBP_DoorRef (.AsBP%20Third%20Person%20Character (Utilities|Casting|CastToBP_ThirdPersonCharacter (Game|GetPlayerCharacter 0))))) "None" "KeepRelative" "KeepRelative" "KeepRelative" true)
  (bind _asbp_third_person_character (Utilities|Casting|CastToBP_ThirdPersonCharacter (Game|GetPlayerCharacter 0)))
  (Class|CableComponent|SetAttachEndtoComponent (Variables|/Game/ThirdPerson/Blueprints/BP_ThirdPersonCharacter.BP_ThirdPersonCharacter_C|GetCableLeftHand _asbp_third_person_character) (Variables|Default|GetSK_GrabpackHand_DefaultOriginalScrewed_Blue) "None"))

(event Custom|AttachHandToPowerReceiver
  (bind _sk_grabpackhand_defaultoriginalscrewed_blue (Variables|Default|GetSK_GrabpackHand_DefaultOriginalScrewed_Blue))
  (bind _sk_grabpackhand_defaultoriginalscrewed_blue_2 (Variables|Default|GetSK_GrabpackHand_DefaultOriginalScrewed_Blue))
  (bind _relativerotation (Variables|/Script/Engine.SceneComponent|GetRelativeRotation _sk_grabpackhand_defaultoriginalscrewed_blue))
  (bind _relativelocation (Variables|/Script/Engine.SceneComponent|GetRelativeLocation _sk_grabpackhand_defaultoriginalscrewed_blue))
  ;[0 0.2344 0.1543] AttachHandToPowerReceiver
  (Transformation|AddRelativeRotation _sk_grabpackhand_defaultoriginalscrewed_blue_2 (Math|Rotator|MakeRotator (.roll _relativerotation) (.pitch _relativerotation) (.yaw _relativerotation)) false false)
  (Transformation|AddRelativeLocation _sk_grabpackhand_defaultoriginalscrewed_blue_2 (Math|Vector|MakeVector (.x _relativelocation) (+ (.y _relativelocation) 15.0) (- (.z _relativelocation) 2e+01)) false false)
  (Components|Animation|PlayAnimation (Variables|Default|GetSK_GrabpackHand_DefaultOriginalScrewed_Blue) "/Game/Hand/SK_Grabpack_HandBlue_Sphere.SK_Grabpack_HandBlue_Sphere" true)
  (Transformation|AttachComponentToComponent (Variables|Default|GetSK_GrabpackHand_DefaultOriginalScrewed_Blue) (Variables|/Game/Blueprints/Mechanics/Poles/BP_PowerReceiver.BP_PowerReceiver_C|GetReceiverMesh (Variables|/Game/ThirdPerson/Blueprints/BP_ThirdPersonCharacter.BP_ThirdPersonCharacter_C|GetBP_PowerReceiverRef (.AsBP%20Third%20Person%20Character (Utilities|Casting|CastToBP_ThirdPersonCharacter (Game|GetPlayerCharacter 0))))) "None" "KeepRelative" "KeepRelative" "KeepRelative" true)
  (Class|CableComponent|SetAttachEndtoComponent (Variables|/Game/ThirdPerson/Blueprints/BP_ThirdPersonCharacter.BP_ThirdPersonCharacter_C|GetCableLeftHand (.AsBP%20Third%20Person%20Character (Utilities|Casting|CastToBP_ThirdPersonCharacter (Game|GetPlayerCharacter 0)))) (Variables|Default|GetSK_GrabpackHand_DefaultOriginalScrewed_Blue) "None"))

(event Custom|AttachHandToLever
  (bind _returnvalue (Game|GetPlayerCharacter 0))
  (bind _sk_grabpackhand_defaultoriginalscrewed_blue (Variables|Default|GetSK_GrabpackHand_DefaultOriginalScrewed_Blue))
  (bind _sk_grabpackhand_defaultoriginalscrewed_blue_2 (Variables|Default|GetSK_GrabpackHand_DefaultOriginalScrewed_Blue))
  (bind _asbp_third_person_character (Utilities|Casting|CastToBP_ThirdPersonCharacter _returnvalue))
  (bind _relativerotation (Variables|/Script/Engine.SceneComponent|GetRelativeRotation _sk_grabpackhand_defaultoriginalscrewed_blue_2))
  (bind _relativelocation (Variables|/Script/Engine.SceneComponent|GetRelativeLocation _sk_grabpackhand_defaultoriginalscrewed_blue_2))
  (bind _bp_leverref (Variables|/Game/ThirdPerson/Blueprints/BP_ThirdPersonCharacter.BP_ThirdPersonCharacter_C|GetBP_LeverRef _asbp_third_person_character))
  ;[1 0.03075 0.06059] AttachHandToLever
  (if (not (Variables|/Game/Blueprints/Mechanics/Lever/BP_Lever.BP_Lever_C|GetIsOpened? _bp_leverref))
    (Transformation|AddRelativeRotation _sk_grabpackhand_defaultoriginalscrewed_blue (Math|Rotator|MakeRotator (+ (.roll _relativerotation) 6e+01) (+ (.pitch _relativerotation) 3e+01) (- (.yaw _relativerotation) 5e+01)) false false)
    (Transformation|AddRelativeLocation _sk_grabpackhand_defaultoriginalscrewed_blue (Math|Vector|MakeVector (+ (.x _relativelocation) 15.0) (+ (.y _relativelocation) 65.0) (+ (.z _relativelocation) 55.0)) false false)
    (Components|Animation|PlayAnimation (Variables|Default|GetSK_GrabpackHand_DefaultOriginalScrewed_Blue) "/Game/Hand/SK_Grabpack_HandBlue_Sphere.SK_Grabpack_HandBlue_Sphere" true)
    (Transformation|AttachComponentToComponent (Variables|Default|GetSK_GrabpackHand_DefaultOriginalScrewed_Blue) (Variables|/Game/Blueprints/Mechanics/Lever/BP_Lever.BP_Lever_C|GetLeverModel _bp_leverref) "None" "KeepRelative" "KeepRelative" "KeepRelative" true)
    (Class|CableComponent|SetAttachEndtoComponent (Variables|/Game/ThirdPerson/Blueprints/BP_ThirdPersonCharacter.BP_ThirdPersonCharacter_C|GetCableLeftHand _asbp_third_person_character) (Variables|Default|GetSK_GrabpackHand_DefaultOriginalScrewed_Blue) "None")))

(event Custom|AttachHandToScanner_Finished
  (bind _sk_grabpackhand_defaultoriginalscrewed_blue (Variables|Default|GetSK_GrabpackHand_DefaultOriginalScrewed_Blue))
  (bind _sk_grabpackhand_defaultoriginalscrewed_blue_2 (Variables|Default|GetSK_GrabpackHand_DefaultOriginalScrewed_Blue))
  (bind _relativerotation (Variables|/Script/Engine.SceneComponent|GetRelativeRotation _sk_grabpackhand_defaultoriginalscrewed_blue_2))
  (bind _relativelocation (Variables|/Script/Engine.SceneComponent|GetRelativeLocation _sk_grabpackhand_defaultoriginalscrewed_blue_2))
  ;[0 0.3326 1] BlueHandScanner
  (bind _returnvalue (Actor|GetActorOfClass "/Game/Blueprints/Mechanics/HandScanner/BP_HandScannerBlue.BP_HandScannerBlue_C"))
  (if (== (Variables|/Game/Blueprints/Mechanics/HandScanner/BP_HandScannerBlue.BP_HandScannerBlue_C|GetScannerForOmni|Blue _returnvalue) 0)
    (Transformation|AddRelativeRotation _sk_grabpackhand_defaultoriginalscrewed_blue (Math|Rotator|MakeRotator (.roll _relativerotation) (.pitch _relativerotation) (+ (.yaw _relativerotation) 3.6e+02)) false false)
    (Transformation|AddRelativeLocation _sk_grabpackhand_defaultoriginalscrewed_blue (Math|Vector|MakeVector (+ (.x _relativelocation) 3.0) (- (.y _relativelocation) 16.0) (- (.z _relativelocation) 21.0)) false false)
    (Utilities|FlowControl|Sequence
      (:then_0
        (Transformation|AttachComponentToComponent _sk_grabpackhand_defaultoriginalscrewed_blue (Variables|/Game/Blueprints/Mechanics/HandScanner/BP_HandScannerBlue.BP_HandScannerBlue_C|GetCube _returnvalue) "None" "KeepRelative" "KeepRelative" "KeepRelative" true))
      (:then_1
        (bind _asbp_third_person_character (Utilities|Casting|CastToBP_ThirdPersonCharacter (Game|GetPlayerCharacter 0)))
        (Variables|/Game/ThirdPerson/Blueprints/BP_ThirdPersonCharacter.BP_ThirdPersonCharacter_C|SetLeftHandAttached? _asbp_third_person_character false)
        (Class|CableComponent|SetAttachEndtoComponent (Variables|/Game/ThirdPerson/Blueprints/BP_ThirdPersonCharacter.BP_ThirdPersonCharacter_C|GetCableLeftHand _asbp_third_person_character) (Variables|Default|GetSK_GrabpackHand_DefaultOriginalScrewed_Blue) "None")))))

(event Custom|HandAttachedToGrabHook
  (bind _sk_grabpackhand_defaultoriginalscrewed_blue (Variables|Default|GetSK_GrabpackHand_DefaultOriginalScrewed_Blue))
  (bind _sk_grabpackhand_defaultoriginalscrewed_blue_2 (Variables|Default|GetSK_GrabpackHand_DefaultOriginalScrewed_Blue))
  (bind _relativerotation (Variables|/Script/Engine.SceneComponent|GetRelativeRotation _sk_grabpackhand_defaultoriginalscrewed_blue_2))
  (bind _relativelocation (Variables|/Script/Engine.SceneComponent|GetRelativeLocation _sk_grabpackhand_defaultoriginalscrewed_blue_2))
  ;[0 0.7661 1] AttachToGrabHook
  (Transformation|AddRelativeRotation _sk_grabpackhand_defaultoriginalscrewed_blue (Math|Rotator|MakeRotator (- (.roll _relativerotation) 9e+01) (.pitch _relativerotation) (- (.yaw _relativerotation) 3.6e+02)) false false)
  (Transformation|AddRelativeLocation _sk_grabpackhand_defaultoriginalscrewed_blue (Math|Vector|MakeVector (- (.x _relativelocation) 3.0) (- (.y _relativelocation) 1e+01) (- (.z _relativelocation) 23.0)) false false)
  (Components|Animation|PlayAnimation _sk_grabpackhand_defaultoriginalscrewed_blue "/Game/Hand/SK_Hand_Grab_GrabHook.SK_Hand_Grab_GrabHook" true)
  (Transformation|AttachComponentToComponent (Variables|Default|GetSK_GrabpackHand_DefaultOriginalScrewed_Blue) (Variables|/Game/Blueprints/Mechanics/GrabHook/BP_GrabHook.BP_GrabHook_C|GetSM_SwingHookHand (Variables|/Game/ThirdPerson/Blueprints/BP_ThirdPersonCharacter.BP_ThirdPersonCharacter_C|GetBP_GrabHookRef (.AsBP%20Third%20Person%20Character (Utilities|Casting|CastToBP_ThirdPersonCharacter (Game|GetPlayerCharacter 0))))) "None" "KeepRelative" "KeepRelative" "KeepRelative" true)
  (Class|CableComponent|SetAttachEndtoComponent (Variables|/Game/ThirdPerson/Blueprints/BP_ThirdPersonCharacter.BP_ThirdPersonCharacter_C|GetCableLeftHand (.AsBP%20Third%20Person%20Character (Utilities|Casting|CastToBP_ThirdPersonCharacter (Game|GetPlayerCharacter 0)))) (Variables|Default|GetSK_GrabpackHand_DefaultOriginalScrewed_Blue) "None"))

(event Custom|AttachHandToScanner
  (bind _returnvalue (Game|GetPlayerCharacter 0))
  (bind _returnvalue_2 (Game|GetPlayerCharacter 0))
  (bind _sk_grabpackhand_defaultoriginalscrewed_blue (Variables|Default|GetSK_GrabpackHand_DefaultOriginalScrewed_Blue))
  (bind _sk_grabpackhand_defaultoriginalscrewed_blue_2 (Variables|Default|GetSK_GrabpackHand_DefaultOriginalScrewed_Blue))
  (bind _asbp_third_person_character (Utilities|Casting|CastToBP_ThirdPersonCharacter _returnvalue))
  (bind _asbp_third_person_character_2 (Utilities|Casting|CastToBP_ThirdPersonCharacter _returnvalue_2))
  (bind _relativerotation (Variables|/Script/Engine.SceneComponent|GetRelativeRotation _sk_grabpackhand_defaultoriginalscrewed_blue))
  (bind _relativelocation (Variables|/Script/Engine.SceneComponent|GetRelativeLocation _sk_grabpackhand_defaultoriginalscrewed_blue))
  (bind _bp_handscannerref (Variables|/Game/ThirdPerson/Blueprints/BP_ThirdPersonCharacter.BP_ThirdPersonCharacter_C|GetBP_HandScannerRef _asbp_third_person_character_2))
  ;[0 0.3326 1] BlueHandScanner
  (if (== (Variables|/Game/Blueprints/Mechanics/HandScanner/BP_HandScannerBlue.BP_HandScannerBlue_C|GetScannerForOmni|Blue _bp_handscannerref) 0)
    (Transformation|AddRelativeRotation _sk_grabpackhand_defaultoriginalscrewed_blue_2 (Math|Rotator|MakeRotator (.roll _relativerotation) (.pitch _relativerotation) (- (.yaw _relativerotation) 3.6e+02)) false false)
    (Transformation|AddRelativeLocation _sk_grabpackhand_defaultoriginalscrewed_blue_2 (Math|Vector|MakeVector (- (.x _relativelocation) 3.0) (+ (.y _relativelocation) 16.0) (+ (.z _relativelocation) 21.0)) false false)
    (Utilities|FlowControl|Sequence
      (:then_0
        (Transformation|AttachComponentToComponent _sk_grabpackhand_defaultoriginalscrewed_blue_2 (Variables|/Game/Blueprints/Mechanics/HandScanner/BP_HandScannerBlue.BP_HandScannerBlue_C|GetCube _bp_handscannerref) "None" "KeepRelative" "KeepRelative" "KeepRelative" true))
      (:then_1
        (Variables|/Game/ThirdPerson/Blueprints/BP_ThirdPersonCharacter.BP_ThirdPersonCharacter_C|SetLeftHandAttached? _asbp_third_person_character true)
        (Class|CableComponent|SetAttachEndtoComponent (Variables|/Game/ThirdPerson/Blueprints/BP_ThirdPersonCharacter.BP_ThirdPersonCharacter_C|GetCableLeftHand _asbp_third_person_character) (Variables|Default|GetSK_GrabpackHand_DefaultOriginalScrewed_Blue) "None")))))

(event Custom|AttachTo_BatteryReceiver
  (bind _sk_grabpackhand_defaultoriginalscrewed_blue (Variables|Default|GetSK_GrabpackHand_DefaultOriginalScrewed_Blue))
  (bind _sk_grabpackhand_defaultoriginalscrewed_blue_2 (Variables|Default|GetSK_GrabpackHand_DefaultOriginalScrewed_Blue))
  (bind _relativerotation (Variables|/Script/Engine.SceneComponent|GetRelativeRotation _sk_grabpackhand_defaultoriginalscrewed_blue))
  (bind _relativelocation (Variables|/Script/Engine.SceneComponent|GetRelativeLocation _sk_grabpackhand_defaultoriginalscrewed_blue))
  ;[0.07146 1 0.2755] AttachHandToBatteryReceiver
  (Transformation|AddRelativeRotation _sk_grabpackhand_defaultoriginalscrewed_blue_2 (Math|Rotator|MakeRotator (+ (.roll _relativerotation) 9e+01) (.pitch _relativerotation) (.yaw _relativerotation)) false false)
  (Transformation|AddRelativeLocation _sk_grabpackhand_defaultoriginalscrewed_blue_2 (Math|Vector|MakeVector (.x _relativelocation) (+ (.y _relativelocation) 15.0) (+ (.z _relativelocation) 17.0)) false false)
  (Components|Animation|PlayAnimation (Variables|Default|GetSK_GrabpackHand_DefaultOriginalScrewed_Blue) "/Game/Hand/SK_GrabpackHand_DefaultOriginalScrewed_Blue_Anim_Armature_handL_grab_smallstraightedge_Anim.SK_GrabpackHand_DefaultOriginalScrewed_Blue_Anim_Armature_handL_grab_smallstraightedge_Anim" true)
  (Transformation|AttachComponentToComponent (Variables|Default|GetSK_GrabpackHand_DefaultOriginalScrewed_Blue) (Variables|/Game/Blueprints/Mechanics/Battery/BP_BatteryReceiver.BP_BatteryReceiver_C|GetBatteryModel (Variables|/Game/ThirdPerson/Blueprints/BP_ThirdPersonCharacter.BP_ThirdPersonCharacter_C|GetBP_BatteryReceiverRef (.AsBP%20Third%20Person%20Character (Utilities|Casting|CastToBP_ThirdPersonCharacter (Game|GetPlayerCharacter 0))))) "None" "KeepRelative" "KeepRelative" "KeepRelative" true)
  (Class|CableComponent|SetAttachEndtoComponent (Variables|/Game/ThirdPerson/Blueprints/BP_ThirdPersonCharacter.BP_ThirdPersonCharacter_C|GetCableLeftHand (.AsBP%20Third%20Person%20Character (Utilities|Casting|CastToBP_ThirdPersonCharacter (Game|GetPlayerCharacter 0)))) (Variables|Default|GetSK_GrabpackHand_DefaultOriginalScrewed_Blue) "None"))

(event Custom|AttachHandToPowerSource
  (bind _sk_grabpackhand_defaultoriginalscrewed_blue (Variables|Default|GetSK_GrabpackHand_DefaultOriginalScrewed_Blue))
  (bind _sk_grabpackhand_defaultoriginalscrewed_blue_2 (Variables|Default|GetSK_GrabpackHand_DefaultOriginalScrewed_Blue))
  (bind _relativerotation (Variables|/Script/Engine.SceneComponent|GetRelativeRotation _sk_grabpackhand_defaultoriginalscrewed_blue))
  (bind _relativelocation (Variables|/Script/Engine.SceneComponent|GetRelativeLocation _sk_grabpackhand_defaultoriginalscrewed_blue))
  ;[0 0.08854 0.05828] AttachHandToPowerSource
  (Transformation|AddRelativeRotation _sk_grabpackhand_defaultoriginalscrewed_blue_2 (Math|Rotator|MakeRotator (.roll _relativerotation) (.pitch _relativerotation) (.yaw _relativerotation)) false false)
  (Transformation|AddRelativeLocation _sk_grabpackhand_defaultoriginalscrewed_blue_2 (Math|Vector|MakeVector (.x _relativelocation) (+ (.y _relativelocation) 36.0) (+ (.z _relativelocation) 43.0)) false false)
  (Components|Animation|PlayAnimation (Variables|Default|GetSK_GrabpackHand_DefaultOriginalScrewed_Blue) "/Game/Hand/SK_Grabpack_HandBlue_Sphere.SK_Grabpack_HandBlue_Sphere" true)
  (Transformation|AttachComponentToComponent (Variables|Default|GetSK_GrabpackHand_DefaultOriginalScrewed_Blue) (Variables|/Game/Blueprints/Mechanics/Poles/BP_PowerSource.BP_PowerSource_C|GetSourceMesh (Variables|/Game/ThirdPerson/Blueprints/BP_ThirdPersonCharacter.BP_ThirdPersonCharacter_C|GetBP_PowerSourceRef (.AsBP%20Third%20Person%20Character (Utilities|Casting|CastToBP_ThirdPersonCharacter (Game|GetPlayerCharacter 0))))) "None" "KeepRelative" "KeepRelative" "KeepRelative" true)
  (Class|CableComponent|SetAttachEndtoComponent (Variables|/Game/ThirdPerson/Blueprints/BP_ThirdPersonCharacter.BP_ThirdPersonCharacter_C|GetCableLeftHand (.AsBP%20Third%20Person%20Character (Utilities|Casting|CastToBP_ThirdPersonCharacter (Game|GetPlayerCharacter 0)))) (Variables|Default|GetSK_GrabpackHand_DefaultOriginalScrewed_Blue) "None"))

(event Custom|HandLever_Anim
  (bind _sk_grabpackhand_defaultoriginalscrewed_blue (Variables|Default|GetSK_GrabpackHand_DefaultOriginalScrewed_Blue))
  (bind _sk_grabpackhand_defaultoriginalscrewed_blue_2 (Variables|Default|GetSK_GrabpackHand_DefaultOriginalScrewed_Blue))
  (bind _relativerotation (Variables|/Script/Engine.SceneComponent|GetRelativeRotation _sk_grabpackhand_defaultoriginalscrewed_blue))
  (bind _relativelocation (Variables|/Script/Engine.SceneComponent|GetRelativeLocation _sk_grabpackhand_defaultoriginalscrewed_blue))
  ;[1 0.03075 0.06059] AttachHandToLever
  (Timeline|HandLever_TL PlayFromStart
    (:Update
      (Utilities|FlowControl|Sequence
        (:then_0
          (Transformation|SetRelativeRotation _sk_grabpackhand_defaultoriginalscrewed_blue_2 (Math|Rotator|MakeRotator (- (.roll _relativerotation) 4e+01) (- (.pitch _relativerotation) 1e+01) (- (.yaw _relativerotation) 6e+01)) false false))
        (:then_1
          (Transformation|SetRelativeLocation _sk_grabpackhand_defaultoriginalscrewed_blue_2 (Math|Vector|MakeVector (- (.x _relativelocation) 1.0) (- (.y _relativelocation) 1.0) (- (.z _relativelocation) 3.7)) false false))))))

(event Custom|HandLever_AnimCancelled
  (bind _sk_grabpackhand_defaultoriginalscrewed_blue (Variables|Default|GetSK_GrabpackHand_DefaultOriginalScrewed_Blue))
  (bind _sk_grabpackhand_defaultoriginalscrewed_blue_2 (Variables|Default|GetSK_GrabpackHand_DefaultOriginalScrewed_Blue))
  (bind _relativerotation (Variables|/Script/Engine.SceneComponent|GetRelativeRotation _sk_grabpackhand_defaultoriginalscrewed_blue))
  (bind _relativelocation (Variables|/Script/Engine.SceneComponent|GetRelativeLocation _sk_grabpackhand_defaultoriginalscrewed_blue))
  ;[1 0.03075 0.06059] AttachHandToLever
  (Timeline|HandLever_TL Reverse
    (:Update
      (Utilities|FlowControl|Sequence
        (:then_0
          (Transformation|SetRelativeRotation _sk_grabpackhand_defaultoriginalscrewed_blue_2 (Math|Rotator|MakeRotator (- (.roll _relativerotation) 4e+01) (- (.pitch _relativerotation) 1e+01) (- (.yaw _relativerotation) 6e+01)) false false))
        (:then_1
          (Transformation|SetRelativeLocation _sk_grabpackhand_defaultoriginalscrewed_blue_2 (Math|Vector|MakeVector (- (.x _relativelocation) 1.0) (- (.y _relativelocation) 1.0) (- (.z _relativelocation) 3.7)) false false))))))

(fn ConstructionScript)